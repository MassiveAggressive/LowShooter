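; Inventory and equipment component that tracks item slots by generated integer ID and moves them between the inventory and per-type, size-limited equipment slots.
; A location map validates each transfer, and changes are broadcast through dispatcher calls.
; Equipping spawns actors for items flagged ShouldBeSpawned; equipment changes re-sum item attributes.
; BeginPlay creates the inventory widget and seeds the inventory with hard-coded DT_Item rows.
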(event EventBeginPlay
  (bind _returnvalue (UserInterface|CreateWidget "/Game/Blueprint/InventoryEquipment/Widget/W_InventoryEquipment.W_InventoryEquipment_C" 0 self))
  (bind _output_get (Variables|Default|SetW_InventoryEquipment _returnvalue))
  (Class|BPIMainWidget|AddWidget(Message) (CallFunction|GetMainWidget) _output_get)
  (for _index (range 0 30)
    (bind _returnvalue_2 (Utilities|GetDataTableRow "/Game/Blueprint/InventoryEquipment/DT_Item.DT_Item" "LF-1")
      (:then
        (Inventory|AddNewItemtoInventory _returnvalue_2))))
  (bind _returnvalue_3 (Utilities|GetDataTableRow "/Game/Blueprint/InventoryEquipment/DT_Item.DT_Item" "SH-1")
    (:then
      (Inventory|AddNewItemtoInventory _returnvalue_3))))

(fn CreateNewID
  (bind _keys (Utilities|Map|Keys (Variables|Default|GetItemSlotLocations)))
  (return (+ (.MaxValue (Math|Integer|MaxOfIntArray _keys)) 1)))

(fn AddNewItemtoInventory
  (params (ItemData :type S%20Item%20Data%20Structure))
  (Inventory|AddItemtoInventory (Utilities|Struct|MakeS_ItemSlot (Inventory|CreateNewID) ItemData)))

(fn AddItemtoInventory
  (params (ItemSlot :type S%20Item%20Slot%20Structure))
  (Utilities|Map|Add (Variables|Inventory|GetInventorySlots) (.ID (Utilities|Struct|BreakS_ItemSlot ItemSlot)) ItemSlot)
  (Utilities|Map|Add (Variables|Default|GetItemSlotLocations) (.ID (Utilities|Struct|BreakS_ItemSlot ItemSlot)) "NewEnumerator0")
  (Default|CallItemAddedtoInventory ItemSlot))

(fn AddItemtoEquipment
  (params (ItemSlot :type S%20Item%20Slot%20Structure))
  (bind _itemdata (Utilities|Struct|BreakS_ItemSlot ItemSlot))
  (bind _equipmenttype (Utilities|Struct|BreakS_ItemData _itemdata))
  (bind (_id _itemdata_2) (Utilities|Struct|BreakS_ItemSlot ItemSlot))
  (bind _keys (Utilities|Map|Keys (Utilities|Struct|BreakS_ItemSlotMap (.Value (Utilities|Map|Find (Variables|Equipment|GetEquipmentSlots) _equipmenttype)))))
  (if (< (Utilities|Array|Length _keys) (.Value (Utilities|Map|Find (Variables|Equipment|GetEquipmentSlotSizes) _equipmenttype)))
    (bind _output_get (LocalVariables|SetItemSlotMapRef (Utilities|Struct|BreakS_ItemSlotMap (.Value (Utilities|Map|Find (Variables|Equipment|GetEquipmentSlots) (.EquipmentType (Utilities|Struct|BreakS_ItemData (.ItemData (Utilities|Struct|BreakS_ItemSlot ItemSlot)))))))))
    (Utilities|Map|Add _output_get _id ItemSlot)
    (Utilities|Map|Add (Variables|Equipment|GetEquipmentSlots) (Utilities|Struct|BreakS_ItemData _itemdata_2) (Utilities|Struct|MakeS_ItemSlotMap (LocalVariables|GetItemSlotMapRef)))
    (if (Utilities|Struct|BreakS_ItemData (Utilities|Struct|BreakS_ItemSlot ItemSlot))
      (CallFunction|SpawnItemActor ItemSlot)
      (Equipment|CalculateAttributes)
      (Utilities|Map|Add (Variables|Default|GetItemSlotLocations) (Utilities|Struct|BreakS_ItemSlot ItemSlot) "NewEnumerator1")
      (Default|CallItemAddedtoEquipment ItemSlot)
      (return true))
    (else
      (return false))))

(fn SendItemtoEquipment
  (params (ItemSlot :type S%20Item%20Slot%20Structure))
  (bind _id (Utilities|Struct|BreakS_ItemSlot ItemSlot))
  (bind (_itemlocation _found) (CallFunction|GetItemLocation _id))
  (if _found
    (switch Utilities|FlowControl|Switch|SwitchonE_ItemLocation _itemlocation
      (:NewEnumerator0
        (bind _added (Equipment|AddItemtoEquipment ItemSlot))
        (if _added
          (Utilities|Map|Remove (Variables|Inventory|GetInventorySlots) (.ID (Utilities|Struct|BreakS_ItemSlot ItemSlot)))
          (Default|CallItemSendedtoEquipment ItemSlot)
          (return true)
          (else
            _)))
      (:NewEnumerator1
        _)))
  (return false))

(fn GetItemLocation
  (params (ItemID :type Integer))
  (bind _itemslotlocations (Variables|Default|GetItemSlotLocations))
  (bind (_value _returnvalue) (Utilities|Map|Find _itemslotlocations ItemID))
  (if _returnvalue
    (return _value true)
    (else
      (return "NewEnumerator0" false))))

(fn SendItemtoInventory
  (params (ItemSlot :type S%20Item%20Slot%20Structure))
  (bind _id (Utilities|Struct|BreakS_ItemSlot ItemSlot))
  (bind (_itemlocation _found) (CallFunction|GetItemLocation _id))
  (if _found
    (switch Utilities|FlowControl|Switch|SwitchonE_ItemLocation _itemlocation
      (:NewEnumerator0
        _)
      (:NewEnumerator1
        (Inventory|AddItemtoInventory ItemSlot)
        (bind _output_get (LocalVariables|SetItemSlotMapRef (Utilities|Struct|BreakS_ItemSlotMap (.Value (Utilities|Map|Find (Variables|Equipment|GetEquipmentSlots) (.EquipmentType (Utilities|Struct|BreakS_ItemData (.ItemData (Utilities|Struct|BreakS_ItemSlot ItemSlot)))))))))
        (Utilities|Map|Remove _output_get (.ID (Utilities|Struct|BreakS_ItemSlot ItemSlot)))
        (Utilities|Map|Add (Variables|Equipment|GetEquipmentSlots) (.EquipmentType (Utilities|Struct|BreakS_ItemData (.ItemData (Utilities|Struct|BreakS_ItemSlot ItemSlot)))) (Utilities|Struct|MakeS_ItemSlotMap (LocalVariables|GetItemSlotMapRef)))
        (Equipment|CalculateAttributes)
        (Default|CallItemSendedtoInventory ItemSlot)
        (return true))))
  (return false))

(fn CalculateAttributes
  (bind _keys (Utilities|Map|Keys (Variables|Equipment|GetEquipmentSlots)))
  (for _array_element _keys
    (bind _output_get (LocalVariables|SetCurrentEquipmentTypeRef _array_element))
    (bind _values (Utilities|Map|Values (Utilities|Struct|BreakS_ItemSlotMap (.Value (Utilities|Map|Find (Variables|Equipment|GetEquipmentSlots) _output_get)))))
    (for _array_element_2 _values
      (bind _output_get_2 (LocalVariables|SetCurrentAttributesRef (.Attributes (Utilities|Struct|BreakS_ItemData (.ItemData (Utilities|Struct|BreakS_ItemSlot _array_element_2))))))
      (bind _keys_2 (Utilities|Map|Keys _output_get_2))
      (for _array_element_3 _keys_2
        (bind _output_get_3 (LocalVariables|SetCurrentAttributeNameRef _array_element_3))
        (if (.ReturnValue (Utilities|Map|Find (LocalVariables|GetCalculatedAttributesRef) _output_get_3))
          (Utilities|Map|Add (LocalVariables|GetCalculatedAttributesRef) (LocalVariables|GetCurrentAttributeNameRef) (+ (.Value (Utilities|Map|Find (LocalVariables|GetCalculatedAttributesRef) (LocalVariables|GetCurrentAttributeNameRef))) (.Value (Utilities|Map|Find (LocalVariables|GetCurrentAttributesRef) (LocalVariables|GetCurrentAttributeNameRef)))))
          (else
            (Utilities|Map|Add (LocalVariables|GetCalculatedAttributesRef) (LocalVariables|GetCurrentAttributeNameRef) (.Value (Utilities|Map|Find (LocalVariables|GetCurrentAttributesRef) (LocalVariables|GetCurrentAttributeNameRef)))))))))
  (bind _output_get_4 (Variables|Default|SetLocalAttributes (LocalVariables|GetCalculatedAttributesRef)))
  (Default|CallAttributesChanged _output_get_4))

(fn SpawnItemActor
  (params (ItemSlot :type S%20Item%20Slot%20Structure))
  (bind _output_get (LocalVariables|SetItemSlotRef ItemSlot))
  (bind _returnvalue (Game|SpawnActorfromClass (Utilities|Struct|BreakS_ItemData (Utilities|Struct|BreakS_ItemSlot _output_get)) (Math|Transform|MakeTransform "0, 0, 0" "0, 0, 0" "1.000000,1.000000,1.000000") "AlwaysSpawn" "MultiplyWithRoot" 0 ItemSlot (Variables|Default|GetItemsInstigator)))
  (bind _output_get_2 (LocalVariables|SetSpawnedItemActorRef _returnvalue))
  (Utilities|Struct|SetmembersinS_ItemSlot (LocalVariables|GetItemSlotRef) _output_get_2))