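; Actor component that stores named attribute values and, on a PlayerController owner, creates an attributes widget and adds it to the main widget.
; Named attribute fields, added directly or from data table rows, are summed per attribute into the final map, broadcasting change events.
; Setters only update existing attributes: SetAttribute fires events after writing, while SetAttributeDirectly is silent.
; Neither setter writes back to the fields, so recalculation replaces those values.
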(event EventBeginPlay
  (Utilities|Casting|CastToPlayerController (Components|GetOwner))
  (bind _returnvalue (UserInterface|CreateWidget "/Game/Blueprint/Attribute/Widget/W_Attributes.W_Attributes_C" 0 self))
  (bind _output_get (Variables|Default|SetW_Attributes _returnvalue))
  (Class|BPIMainWidget|AddWidget(Message) (CallFunction|GetMainWidget) _output_get))

(fn GetAttribute
  (params (AttributeName :type Name))
  (bind _attributes (Variables|Default|GetAttributes))
  (bind (_value _returnvalue) (Utilities|Map|Find _attributes AttributeName))
  (return _value _returnvalue))

(fn GetAttributes
  (return (Variables|Default|GetAttributes)))

(fn SetAttribute
  (params (AttributeName :type Name) (AttributeValue :type Float%20%28double-precision%29))
  (bind _attributes (Variables|Default|GetAttributes))
  (bind (_value _returnvalue) (Utilities|Map|Find _attributes AttributeName))
  (if _returnvalue
    (LocalVariables|SetAttributeOldValueRef _value)
    (Utilities|Map|Add (Variables|Default|GetAttributes) AttributeName AttributeValue)
    (Default|CallAttributeAbouttoChange AttributeName)
    (Default|CallAttributeChanged AttributeName (LocalVariables|GetAttributeOldValueRef) (.Value (Utilities|Map|Find (Variables|Default|GetAttributes) AttributeName)))))

(fn SetAttributeDirectly
  (params (AttributeName :type Name) (AttributeValue :type Float%20%28double-precision%29))
  (if (.ReturnValue (Utilities|Map|Find (Variables|Default|GetAttributes) AttributeName))
    (Utilities|Map|Add (Variables|Default|GetAttributes) AttributeName AttributeValue)))

(fn AddAttributesField
  (params (AttributesFieldName :type Name) (Attributes :type Map%20of%20Names%20to%20Reals))
  (Utilities|Map|Add (Variables|Default|GetAttributesFields) AttributesFieldName (Utilities|Struct|MakeS_AttributesMap Attributes))
  (CallFunction|CalculateAttributes))

(fn InitializeAttributesbyDataTable
  (params (AttributesFieldsName :type Name) (DataTableRowHandle :type Data%20Table%20Row%20Handle%20Structure%20%28by%20ref%29))
  (bind (_datatable _rowname) (Utilities|Struct|BreakDataTableRowHandle DataTableRowHandle))
  (bind _returnvalue (Utilities|GetDataTableRow _datatable _rowname)
    (:then
      (Utilities|Map|Add (Variables|Default|GetAttributesFields) AttributesFieldsName (Utilities|Struct|MakeS_AttributesMap (Utilities|Struct|BreakS_AttributesMap _returnvalue)))
      (CallFunction|CalculateAttributes))))

(fn CalculateAttributes
  (bind _keys (Utilities|Map|Keys (Variables|Default|GetAttributesFields)))
  (for _array_element _keys
    (LocalVariables|SetCurrentAttributeFieldNameRef _array_element)
    (bind _output_get (LocalVariables|SetCurrentCalculatedAttributesRef (Utilities|Struct|BreakS_AttributesMap (.Value (Utilities|Map|Find (Variables|Default|GetAttributesFields) _array_element)))))
    (bind _keys_2 (Utilities|Map|Keys _output_get))
    (for _array_element_2 _keys_2
      (bind _output_get_2 (LocalVariables|SetCurrentAttributeNameRef _array_element_2))
      (if (.ReturnValue (Utilities|Map|Find (LocalVariables|GetCalculatedAttributesRef) _output_get_2))
        (Utilities|Map|Add (LocalVariables|GetCalculatedAttributesRef) (LocalVariables|GetCurrentAttributeNameRef) (+ (.Value (Utilities|Map|Find (LocalVariables|GetCalculatedAttributesRef) (LocalVariables|GetCurrentAttributeNameRef))) (.Value (Utilities|Map|Find (LocalVariables|GetCurrentCalculatedAttributesRef) (LocalVariables|GetCurrentAttributeNameRef)))))
        (else
          (Utilities|Map|Add (LocalVariables|GetCalculatedAttributesRef) (LocalVariables|GetCurrentAttributeNameRef) (.Value (Utilities|Map|Find (LocalVariables|GetCurrentCalculatedAttributesRef) (LocalVariables|GetCurrentAttributeNameRef))))))))
  (LocalVariables|SetOldAttributesRef (Variables|Default|GetAttributes))
  (bind _output_get_3 (Variables|Default|SetAttributes (LocalVariables|GetCalculatedAttributesRef)))
  (bind _keys_3 (Utilities|Map|Keys _output_get_3))
  (for _array_element_3 _keys_3
    (Default|CallAttributeChanged _array_element_3 (.Value (Utilities|Map|Find (LocalVariables|GetOldAttributesRef) _array_element_3)) (.Value (Utilities|Map|Find (Variables|Default|GetAttributes) _array_element_3))))
  (Default|CallAttributesChanged (Variables|Default|GetAttributes)))