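; Attribute driver Blueprint that keeps an owner's Health within valid bounds and signals death.
; It overrides AttributeAboutToChange, calling the parent first, then reacting only to the Health attribute.
; It reads Health and MaxHealth from the attributes container component, clamps Health between zero and MaxHealth, and writes it back through SetAttributeDirectly.
; When the clamped value equals zero, it calls CallOwnerAboutToDie.
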(event EventBeginPlay
  (|CallParentFunction) ; This node is disabled and will not be called.\nDrag off pins to build functionality.
)

(event EventTick
  (params (DeltaSeconds :type Float%20%28single-precision%29)))

(fn AttributeAbouttoChange
  (params (AttributeName :type Name :default "None"))
  (bind _attributescontainercomponent (Variables|Default|GetAttributesContainerComponent))
  (|CallParentFunction AttributeName)
  (if (== AttributeName "Health")
    (bind _output_get (LocalVariables|SetHealthAttributeNewValueRef (Math|Float|Clamp(Float) (.AttributeValue (Default|GetAttribute _attributescontainercomponent "Health")) 0.0 (.AttributeValue (Default|GetAttribute _attributescontainercomponent "MaxHealth")))))
    (Default|SetAttributeDirectly (Variables|Default|GetAttributesContainerComponent) "Health" _output_get)
    (if (== (LocalVariables|GetHealthAttributeNewValueRef) 0.0)
      (Default|CallOwnerAbouttoDie))))