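; BP_AttributesDriver registers a field of default attributes with its owner's BP_AttributesContainer and listens for attribute changes, apparently as a base for attribute-specific drivers.
; On BeginPlay it finds the container, binds its about-to-change and changed events, then adds the named field.
; AttributeAboutToChange and AttributeChanged are empty stubs, so this asset applies no reaction logic itself.
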(event EventBeginPlay
  (bind _output_get (Variables|Default|SetAttributesContainerComponent (Actor|GetComponentbyClass (Components|GetOwner) "/Game/Blueprint/Attribute/BP_AttributesContainer.BP_AttributesContainer_C")))
  (EventDispatchers|BindEventtoAttributeAbouttoChange _output_get (EventDispatchers|CreateEvent :!event AttributeAbouttoChange))
  (EventDispatchers|BindEventtoAttributeChanged _output_get (EventDispatchers|CreateEvent :!event AttributeChanged))
  (Default|AddAttributesField (Variables|Default|GetAttributesContainerComponent) (Variables|Default|GetAttributeFieldName) (Variables|Default|GetDefaultAttributes)))

(fn AttributeAbouttoChange
  (params (AttributeName :type Name)))

(fn AttributeChanged
  (params (AttributeName :type Name) (AttributeOldValue :type Float%20%28double-precision%29) (AttributeNewValue :type Float%20%28double-precision%29)))