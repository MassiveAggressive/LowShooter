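; BP_DamageAttributesDriver is an attribute driver that keeps Damage and FireRate equal to their MaxDamage and MaxFireRate attributes.
; It overrides the about-to-change and changed callbacks, calling the parent and then a shared equalize function in both.
; That function switches on the attribute name and, for either max attribute, writes its value directly to the matching attribute through the AttributesContainerComponent.
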(fn AttributeAbouttoChange
  (params (AttributeName :type Name :default "None"))
  (|CallParentFunction AttributeName)
  (CallFunction|EqualizeDamageAttributes AttributeName))

(fn EqualizeDamageAttributes
  (params (AttributeName :type Name))
  (bind _attributescontainercomponent (Variables|Default|GetAttributesContainerComponent))
  (bind _attributescontainercomponent_2 (Variables|Default|GetAttributesContainerComponent))
  (switch name AttributeName
    (:MaxDamage
      (Default|SetAttributeDirectly _attributescontainercomponent_2 "Damage" (.AttributeValue (Default|GetAttribute _attributescontainercomponent_2 "MaxDamage"))))
    (:MaxFireRate
      (Default|SetAttributeDirectly _attributescontainercomponent "FireRate" (.AttributeValue (Default|GetAttribute _attributescontainercomponent "MaxFireRate"))))))

(fn AttributeChanged
  (params (AttributeName :type Name :default "None") (AttributeOldValue :type Float%20%28double-precision%29) (AttributeNewValue :type Float%20%28double-precision%29))
  (|CallParentFunction AttributeName AttributeOldValue AttributeNewValue)
  (CallFunction|EqualizeDamageAttributes AttributeName))