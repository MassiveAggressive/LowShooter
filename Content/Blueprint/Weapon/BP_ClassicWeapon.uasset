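; BP_ClassicWeapon is a weapon Blueprint that fires one BP_BulletBase projectile from each of its barrels.
; Its Shoot override calls the parent, then spawns bullets along each barrel's rotation, always spawning regardless of collision and passing on the Instigator.
; Each spawn point is pushed forward along the barrel in proportion to the Latency argument, offsetting the bullet for delay using a fixed speed factor.
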(fn ConstructionScript
  (|CallParentFunction))

(fn Shoot
  (params (Latency :type Float%20%28double-precision%29))
  (|CallParentFunction Latency)
  (for _array_element (Variables|Default|GetBarrels)
    (Game|SpawnActorfromClass "/Game/Blueprint/Weapon/Bullet/BP_BulletBase.BP_BulletBase_C" (Math|Transform|MakeTransform (+ (Transformation|GetWorldLocation _array_element) (* (Math|Vector|GetForwardVector _array_element) Latency 3e+03)) (Transformation|GetWorldRotation _array_element) "1.000000,1.000000,1.000000") "AlwaysSpawn" "MultiplyWithRoot" 0 (Variables|Default|GetInstigator))))