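; Base weapon actor that handles fire-rate timing and barrel layout, with Shoot only clearing shot availability and spawning no projectile.
; StartShooting fires immediately if ready and enables Tick, which accumulates time and repeats Shoot with leftover latency for frame-rate-independent fire, then turns itself off once stopped and cooled down.
; The Construction Script rebuilds centered, fanned arrow components as barrels.
; An Instigator attribute-change binding keeps fire rate current.
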(event EventBeginPlay
  (Variables|Default|SetFireDuration (/ 1.0 (Variables|Default|GetFireRate)))
  (bind _attributecontainer (Class|BPIAttributes|GetAttributesContainer(Message) (Variables|Actor|GetInstigator)))
  (EventDispatchers|BindEventtoAttributeChanged _attributecontainer (EventDispatchers|CreateEvent :!event AttributeChanged)))

(event EventTick
  (params (DeltaSeconds :type Float%20%28single-precision%29))
  (if (Variables|Default|GetCountThisFrame)
    (bind _output_get (Variables|Default|SetTimePool (+ (Variables|Default|GetTimePool) (Utilities|Time|GetWorldDeltaSeconds))))
    (if (>= _output_get (Variables|Default|GetFireDuration))
      (if (Variables|Default|GetShooting)
        (CallFunction|HandleTimePool)
        (else
          (Variables|Default|SetTimePool 0.0)
          (Variables|Default|SetShootAvailable true)
          (Variables|Default|SetCountThisFrame false)
          (Actor|Tick|SetActorTickEnabled false))))
    (else
      (Variables|Default|SetCountThisFrame true))))

(fn ConstructionScript
  (CallFunction|UpdateBarrels))

(fn StartShooting
  (if (> (Variables|Default|GetFireDuration) 0.0)
    (if (Variables|Default|GetShootAvailable)
      (CallFunction|Shoot 0.0))
    (Variables|Default|SetShooting true)
    (Actor|Tick|SetActorTickEnabled true)))

(fn StopShooting
  (Variables|Default|SetShooting false))

(fn HandleTimePool
  (while (>= (Variables|Default|GetTimePool) (Variables|Default|GetFireDuration))
    (bind _output_get (Variables|Default|SetTimePool (- (Variables|Default|GetTimePool) (Variables|Default|GetFireDuration))))
    (CallFunction|Shoot _output_get)))

(fn Shoot
  (params (Latency :type Float%20%28double-precision%29))
  (Variables|Default|SetShootAvailable false))

(fn UpdateBarrels
  (for _array_element (Variables|Barrel|GetBarrels)
    (Components|DestroyComponent _array_element))
  (Utilities|Array|Clear (Variables|Barrel|GetBarrels))
  (for _index (range 0 (- (Variables|Barrel|GetBarrelsCount) 1))
    (bind _returnvalue (AddComponent|AddArrowComponent false (Math|Transform|MakeTransform (Math|Vector|MakeVector 0.0 (- (* _index (Variables|Barrel|GetBarrelsDistance)) (* (- (Variables|Barrel|GetBarrelsCount) 1) (Variables|Barrel|GetBarrelsDistance) 0.5)) 0.0) (Math|Rotator|MakeRotator 0.0 0.0 (- (* _index (Variables|Barrel|GetBarrelsDegree)) (* (- (Variables|Barrel|GetBarrelsCount) 1) (Variables|Barrel|GetBarrelsDegree) 0.5))) "1.000000,1.000000,1.000000")))
    (Utilities|Array|Add (Variables|Barrel|GetBarrels) _returnvalue)))

(fn AttributeChanged
  (params (AttributeName :type Name) (AttributeOldValue :type Float%20%28double-precision%29) (AttributeNewValue :type Float%20%28double-precision%29))
  (switch name AttributeName
    (:FireRate
      (bind _output_get (Variables|Default|SetFireRate AttributeNewValue))
      (Variables|Default|SetFireDuration (/ 1.0 _output_get)))))