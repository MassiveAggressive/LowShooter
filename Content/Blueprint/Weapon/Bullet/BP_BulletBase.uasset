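; Base projectile Blueprint for bullets that fly forward, spark on impact and damage actors that have attributes.
; The first Tick activates ProjectileMovement with a fixed local forward velocity, then disables ticking.
; On box hit, it spawns tinted Niagara sparks, subtracts the instigator's Damage attribute from the target's Health through BPI_Attributes, and destroys itself.
; The construction script applies the same BulletColor to the mesh through a dynamic material.
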(event OnComponentHit(Box)
  (params (HitComponent :type Primitive%20Component%20Object%20Reference) (OtherActor :type Actor%20Object%20Reference) (OtherComp :type Primitive%20Component%20Object%20Reference) (NormalImpulse :type Vector :default "0, 0, 0") (Hit :type Hit%20Result%20Structure%20%28by%20ref%29))
  (bind (_bblockinghit _binitialoverlap _time _distance _location _impactpoint _normal _impactnormal) (Collision|BreakHitResult Hit))
  (bind _returnvalue (Niagara|SpawnSystematLocation "/Game/Asset/Particle/NS_Sparks.NS_Sparks" _impactpoint (Math|Rotator|MakeRotfromX _impactnormal)))
  (Effects|Components|ParticleSystem|SetColorParameter _returnvalue "Color" (Variables|Default|GetBulletColor))
  (if (Utilities|DoesObjectImplementInterface OtherActor "/Game/Blueprint/Attribute/Interface/BPI_Attributes.BPI_Attributes_C")
    (bind _attributevalue (Class|BPIAttributes|GetAttribute(Message) OtherActor "Health"))
    (Class|BPIAttributes|SetAttribute(Message) OtherActor "Health" (- _attributevalue (.AttributeValue (CallFunction|GetAttribute (Game|GetInstigator) "Damage"))))
    (Actor|DestroyActor)
    (else
      (Actor|DestroyActor))))

(event EventTick
  (params (DeltaSeconds :type Float%20%28single-precision%29))
  (bind _projectilemovement (Variables|Default|GetProjectileMovement))
  (Components|Activation|Activate _projectilemovement false)
  (Game|Components|ProjectileMovement|SetVelocityinLocalSpace _projectilemovement "3000.000000,0.000000,0.000000")
  (Actor|Tick|SetActorTickEnabled false))

(fn ConstructionScript
  (bind _returnvalue (Rendering|Material|CreateDynamicMaterialInstance (Variables|Default|GetCube) 0 "/Game/Blueprint/Weapon/Bullet/Material/MI_Bullet.MI_Bullet" "None" :!class /Script/Engine.PrimitiveComponent))
  (Rendering|Material|SetVectorParameterValue _returnvalue "Color" (Variables|Default|GetBulletColor) :!class /Script/Engine.MaterialInstanceDynamic))