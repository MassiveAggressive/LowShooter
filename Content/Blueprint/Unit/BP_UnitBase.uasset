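; BP_UnitBase is a base unit Blueprint that exposes attributes and mesh sockets.
; On possession it caches the attribute container and health driver components from the new controller, then initializes attributes from its default data table row.
; Attribute get and set calls forward to that controller-owned container, while socket queries resolve against the Cube mesh in world space.
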(event EventSetAttribute
  (params (AttributeName :type Name :default "None") (AttributeValue :type Float%20%28double-precision%29))
  (Default|SetAttribute (Variables|Default|GetAttributesContainerComponent) AttributeName AttributeValue))

(event EventBeginPlay)

(event EventPossessed
  (params (NewController :type Controller%20Object%20Reference))
  (bind _output_get (Variables|Default|SetAttributesContainerComponent (Actor|GetComponentbyClass NewController "/Game/Blueprint/Attribute/BP_AttributesContainer.BP_AttributesContainer_C")))
  (Variables|Default|SetHealthAttributeDriver (Actor|GetComponentbyClass NewController "/Game/Blueprint/Attribute/BP_HealthAttributesDriver.BP_HealthAttributesDriver_C"))
  (Default|InitializeAttributesbyDataTable _output_get "Default" (Variables|Default|GetDefaultAttributes)))

(fn ConstructionScript)

(fn GetAllSocketNames
  (return (Transformation|GetAllSocketNames (Variables|Default|GetCube))))

(fn GetAttribute
  (params (AttributeName :type Name :default "None"))
  (bind _attributescontainercomponent (Variables|Default|GetAttributesContainerComponent))
  (bind (_attributevalue _found) (Default|GetAttribute _attributescontainercomponent AttributeName))
  (return _attributevalue _found))

(fn GetAttributesContainer
  (return (Variables|Default|GetAttributesContainerComponent)))

(fn GetSocket
  (params (SocketName :type Name :default "None"))
  (return (Variables|Default|GetCube) (Transformation|GetSocketTransform (Variables|Default|GetCube) SocketName "RTS_World")))