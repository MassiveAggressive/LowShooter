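; Custom movement component that moves and rotates its owning actor every tick.
; AddMovementInput stores a normalized direction, which Move applies as a non-swept world offset at the current speed, then clears.
; RotateToTargetRotation starts a constant-speed interpolation from the owner's yaw toward a target rotation, stopped by a per-frame yaw-delta check.
; AddRotateInput is empty, and the look-at-location rotation logic is never run.
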(event EventTick
  (params (DeltaSeconds :type Float%20%28single-precision%29))
  (CallFunction|Move)
  (if (Variables|Rotation|GetRotating)
    (CallFunction|Rotate)))

(fn AddMovementInput
  (params (Input :type Vector))
  (Variables|Movement|SetMovementInput (Math|Vector|Normalize Input)))

(fn Move
  (Transformation|AddActorWorldOffset (Components|GetOwner) (* (Variables|Movement|GetMovementInput) (Variables|Movement|GetCurrentMovementSpeed) (Utilities|Time|GetWorldDeltaSeconds)))
  (Variables|Movement|SetMovementInput "0, 0, 0"))

(fn AddRotateInput)

(fn Rotate
  (bind _returnvalue (Components|GetOwner))
  (if (Variables|Rotation|GetRotatingToTarget)
    (switch Utilities|FlowControl|Switch|SwitchonE_RotationTargetType (Variables|Rotation|GetRotationTargetType)
      (:NewEnumerator0
        (Transformation|SetActorRotation _returnvalue (Class|KismetMathLibrary|RInterptoConstant (Math|Rotator|MakeRotator 0.0 0.0 (.yaw (Transformation|GetActorRotation _returnvalue))) (Variables|Rotation|GetTargetRotationToRotate) (Utilities|Time|GetWorldDeltaSeconds) (Variables|Rotation|GetCurrentRotationSpeed)))
        (if (> (* (Variables|Rotation|GetCurrentRotationSpeed) (Utilities|Time|GetWorldDeltaSeconds)) (.yaw (Math|Rotator|Delta(Rotator) (Math|Rotator|MakeRotator 0.0 0.0 (.yaw (Transformation|GetActorRotation (Components|GetOwner)))) (Variables|Rotation|GetTargetRotationToRotate))))
          (Variables|Rotation|SetRotatingToTarget false)
          (Variables|Rotation|SetRotating false))))))

(fn RotatetoTargetRotation
  (params (TargetRotation :type Rotator))
  (Variables|Rotation|SetTargetRotationToRotate TargetRotation)
  (Variables|Rotation|SetRotationTargetType "NewEnumerator0")
  (Variables|Rotation|SetRotatingToTarget true)
  (Variables|Rotation|SetRotating true))