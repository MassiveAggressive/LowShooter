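; Player-controlled unit that moves from input, turns to face a hit location and shoots a weapon.
; On BeginPlay it adds the general Enhanced Input mapping, then spawns a classic weapon and attaches it to its weapon socket.
; A movement component receives move input and, every tick, a yaw-only look-at rotation toward the hit location.
; Left mouse press and release start and stop the weapon's shooting.
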(event Input|EnhancedActionEvents|EnhancedInputActionIA_Move
  (params (ActionValue :type Vector%202D%20Structure) (ElapsedSeconds :type Float%20%28double-precision%29) (TriggeredSeconds :type Float%20%28double-precision%29) (InputAction :type Input%20Action%20Object%20Reference :default "/Game/Input/IA_Move.IA_Move"))
  (:Triggered
    (Default|AddMovementInput (Variables|Default|GetBP_MovementComponent) (Math|Vector|MakeVector (.x ActionValue) (.y ActionValue) 0.0) :!label _label))
  (:Started
    (goto _label))
  (:Completed
    (goto _label)))

(event EventBeginPlay
  (|CallParentFunction)
  (Input|AddMappingContext (PlayerController|LocalPlayerSubsystems|GetEnhancedInputLocalPlayerSubsystem (Game|GetPlayerController 0)) "/Game/Input/IMC_General.IMC_General" 0 "(bIgnoreAllPressedKeysUntilRelease=True,bForceImmediately=False,bNotifyUserSettings=False)")
  (bind _returnvalue (Game|SpawnActorfromClass :Class "/Game/Blueprint/Weapon/BP_ClassicWeapon.BP_ClassicWeapon_C" :SpawnTransform (Transformation|GetWorldTransform (Variables|Default|GetWeaponSocket)) :CollisionHandlingOverride "AlwaysSpawn" :TransformScaleMethod "MultiplyWithRoot" :Instigator self))
  (bind _output_get (Variables|Default|SetWeapon _returnvalue))
  (Transformation|AttachComponentToComponent _output_get (Variables|Default|GetWeaponSocket) "None" "SnapToTarget" "SnapToTarget" "KeepWorld" true))

(event EventTick
  (params (DeltaSeconds :type Float%20%28single-precision%29))
  (Default|RotatetoTargetRotation (Variables|Default|GetBP_MovementComponent) (Math|Rotator|MakeRotator 0.0 0.0 (.yaw (Math|Rotator|FindLookatRotation (Transformation|GetActorLocation) (CallFunction|GetHitLocation))))))

(event Input|MouseEvents|LeftMouseButton
  (params (Key :type Key%20Structure :default "None"))
  (bind _weapon (Variables|Default|GetWeapon))
  (:Pressed
    (Default|StartShooting _weapon))
  (:Released
    (Default|StopShooting _weapon)))

(fn ConstructionScript
  (|CallParentFunction))